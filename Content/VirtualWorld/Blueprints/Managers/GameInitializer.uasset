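; GameInitializer is a manager actor that boots the virtual world's Photon Cloud networking and UI on BeginPlay.
; It caches the PhotonHandler, game instance and player controller, initializes the handler with the latter two, then spawns BP_ChatHandler.
; It shows the mouse cursor and adds the PhotonHandlerUI and VC_Enabler widgets to the viewport.
; Keys 1 and 2 recreate and remove those widgets.
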(event Custom|DisplayPhotonUI
  (Variables|/Script/Engine.PlayerController|SetbShowMouseCursor (Game|GetPlayerController 0) true)
  (bind _returnvalue (UserInterface|CreateWidget "/Game/VirtualWorld/AgoraVoiceChat/VC_Enabler.VC_Enabler_C"))
  (bind _returnvalue_2 (UserInterface|CreateWidget "/Game/VirtualWorld/Blueprints/Widgets/PhotonHandlerUI.PhotonHandlerUI_C"))
  (UserInterface|Viewport|AddtoViewport _returnvalue_2 0))

(event EventBeginPlay
  (Utilities|FlowControl|Sequence
    (:then_0
      (CallFunction|InitializeVariables))
    (:then_1
      (Game|SpawnActorfromClass "/Game/VirtualWorld/Blueprints/Managers/BP_ChatHandler.BP_ChatHandler_C" (Math|Transform|MakeTransform "0, 0, 0" "0, 0, 0" "1.000000,1.000000,1.000000") "Undefined" 0 "GroupChat" 0))
    (:then_2
      (CallFunction|DisplayPhotonUI))
    (:then_3
      (Input|EnableInput (Variables|Default|GetPlayerController)))))

(event Input|KeyboardEvents|2
  (params (Key :type Key%20Structure :default "None"))
  (:Pressed
    (Widget|RemovefromParent (stale Custom|DisplayPhotonUI _returnvalue))))

(event Input|KeyboardEvents|1
  (params (Key :type Key%20Structure :default "None"))
  (:Pressed
    (CallFunction|DisplayPhotonUI)))

(fn ConstructionScript)

(fn InitializeVariables
  (Utilities|FlowControl|Sequence
    (:then_0
      (bind _asphoton_handler (Utilities|Casting|CastToPhotonHandler (Class|PhotonCloudSubsystem|GetPhotonCloudAPI (Subsystems|GetPhotonCloudSubsystem))))
      (Variables|Default|SetPhotonHandler _asphoton_handler))
    (:then_1
      (bind _asgi_virtual_world (Utilities|Casting|CastToGI_VirtualWorld (Game|GetGameInstance)))
      (Variables|Default|SetVW_GameInstance _asgi_virtual_world))
    (:then_2
      (bind _asplayer_controller_bp (Utilities|Casting|CastToPlayerControllerBP (Game|GetPlayerController 0)))
      (Variables|Default|SetPlayerController _asplayer_controller_bp))
    (:then_3
      (Default|InitializePhotonHandler (Variables|Default|GetPhotonHandler) (Variables|Default|GetVW_GameInstance) (Variables|Default|GetPlayerController)))))