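; Notification manager actor for the virtual world that requests invitations from the API_Manager, with the response handler still empty.
; On BeginPlay it finds the API_Manager, caches the game instance, starts a delayed fetch and binds to the invitations response event.
; Despite its name, LoopForNotifications fetches only once after the delay, using a hard-coded placeholder username instead of the logged-in user.
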(event Custom|LoopForNotifications
  (Utilities|FlowControl|Delay 5.0)
  (Default|FetchInvitations (Variables|Default|GetAPI_Manager) "qqq"))

(event Custom|OnNotificationsFetched
  (params (NotificationText :type String)))

(event EventBeginPlay
  (bind _outactors (Actor|GetAllActorsOfClass "/Game/VirtualWorld/Blueprints/APIs/API_Manager.API_Manager_C"))
  (Variables|Default|SetAPI_Manager (Utilities|Array|Get(acopy) _outactors))
  (bind _asgi_virtual_world (Utilities|Casting|CastToGI_VirtualWorld (Game|GetGameInstance)))
  (Variables|Default|SetGameInstanceVW _asgi_virtual_world)
  (CallFunction|LoopforNotifications)
  (EventDispatchers|BindEventtoOnInvitationsFetchResponse (Variables|Default|GetAPI_Manager) (delegate Custom|OnNotificationsFetched)))

(event Collision|EventActorBeginOverlap
  (params (OtherActor :type Actor%20Object%20Reference)))

(event EventTick
  (params (DeltaSeconds :type Float%20%28single-precision%29)))

(fn ConstructionScript)