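; BP_InputManager handles mouse input for toggling the avatar's interaction widget in the virtual world.
; On BeginPlay it enables input and caches the player pawn as a Bp_avatar reference.
; A right-click over any pawn under the cursor prints its name and toggles that cached avatar's widget visibility.
; Every tick it turns the widget toward the follow camera using look-at yaw and roll, with pitch fixed at zero.
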(event EventTick
  (params (DeltaSeconds :type Float%20%28single-precision%29))
  (bind _bp_avatar_ref (Variables|Default|GetBp_Avatar_Ref))
  (bind _bp_avatar_ref_2 (Variables|Default|GetBp_Avatar_Ref))
  (bind _followcamera (Variables|/Game/ThirdPersonBP/Blueprints/ThirdPersonCharacter.ThirdPersonCharacter_C|GetFollowCamera _bp_avatar_ref_2))
  (bind _widget (Variables|/Game/VirtualWorld/Blueprints/Avatars/Bp_avatar.Bp_avatar_C|GetWidget _bp_avatar_ref))
  (bind _returnvalue (Transformation|GetWorldLocation _widget))
  (bind _returnvalue_2 (Transformation|GetWorldLocation _followcamera))
  (bind _returnvalue_3 (Math|Rotator|FindLookatRotation _returnvalue _returnvalue_2))
  (bind (_roll _pitch _yaw) (Math|Rotator|BreakRotator _returnvalue_3))
  ;[1 1 1] CAMERA LOOK AT FUNTIONALITY
  (Transformation|SetWorldRotation (Variables|/Game/VirtualWorld/Blueprints/Avatars/Bp_avatar.Bp_avatar_C|GetWidget (Variables|Default|GetBp_Avatar_Ref)) (Math|Rotator|MakeRotator (- _roll 0.0) 0.0 (- _yaw 0.0)) false false))

(event EventBeginPlay
  ;[1 1 1] ENABLE INPUT AND SET BP_AVATAR REFERENCE
  (Input|EnableInput (Game|GetPlayerController 0))
  (bind _asbp_avatar (Utilities|Casting|CastToBp_avatar (Game|Player|GetPlayerPawn 0)))
  (Variables|Default|SetBp_Avatar_Ref _asbp_avatar))

(event Input|MouseEvents|RightMouseButton
  (params (Key :type Key%20Structure))
  (bind _returnvalue (Game|GetPlayerController 0))
  (bind _array (Utilities|Array|MakeArray "ObjectTypeQuery3"))
  (bind _hitresult (Class|PlayerController|GetHitResultUnderCursorforObjects _returnvalue _array true))
  (bind _hitactor (Collision|BreakHitResult _hitresult))
  ;[1 1 1] INTERACTIONS WIDGET TOGGLE
  (:Pressed
    (Utilities|IsValid _hitactor
      (:Is%20Valid
        (Development|PrintString (Utilities|GetDisplayName _hitactor))
        (if (Class|WidgetComponent|IsWidgetVisible (Variables|/Game/VirtualWorld/Blueprints/Avatars/Bp_avatar.Bp_avatar_C|GetWidget (Variables|Default|GetBp_Avatar_Ref)))
          (Rendering|SetVisibility (Variables|/Game/VirtualWorld/Blueprints/Avatars/Bp_avatar.Bp_avatar_C|GetWidget (Variables|Default|GetBp_Avatar_Ref)) false false)
          (else
            (Rendering|SetVisibility (Variables|/Game/VirtualWorld/Blueprints/Avatars/Bp_avatar.Bp_avatar_C|GetWidget (Variables|Default|GetBp_Avatar_Ref)) true false)))))))

(fn ConstructionScript)