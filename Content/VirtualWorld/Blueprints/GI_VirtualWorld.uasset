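; Game instance for a virtual world, holding session state: logged-in user, avatar, open panel, meeting and property selections.
; Resets the Photon Cloud session, showing a can't-connect panel on failure; after login it connects, then opens the user's numbered InteriorPreset personal space.
; Space loading resolves the avatar from an ID map before opening the level.
; Also manages single-panel UI, seeds a hardcoded property listing and logs seller, agent and buyer selections.
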(event Custom|OnUserLoggedInSuccessfully
  (CallFunction|ConnectwithPhoton))

(event Custom|ClosePanel
  (Variables|/Script/Engine.PlayerController|SetbShowMouseCursor (Game|GetPlayerController 0) false)
  (Viewport|RemoveAllWidgets))

(event Custom|LoadInDefaultSpace
  (CallFunction|LoadCurrentUserinSpace "PersonalSpace"))

(event Custom|OnPhotonFailed
  (CallFunction|OpenPanel "/Game/VirtualWorld/Blueprints/Widgets/AccountDetails/InGameWidgets/W_PhotonCantConnect.W_PhotonCantConnect_C" true))

(event Custom|ResetGameSession
  (Variables|Default|SetCurrentSelectedAvatar "/Game/MetaHumans/Aoi/BP_Aoi.BP_Aoi_C")
  (Variables|Default|SetCurrentLoggedInUser "")
  (Variables|Default|SetCurrentOpenedPanel 0)
  (Variables|Default|SetCurrentJoinedMeetingData "")
  (CallFunction|InitializeGameInstance))

(event Custom|InitializeGameInstance
  (bind _asphoton_cloud_object_api_bp (Utilities|Casting|CastToPhotonCloudObjectAPI_BP (Class|PhotonCloudSubsystem|GetPhotonCloudAPI (Subsystems|GetPhotonCloudSubsystem))))
  (Default|ResetPhotonSession _asphoton_cloud_object_api_bp)
  (EventDispatchers|AssignOnPhotonConnectionFailed _asphoton_cloud_object_api_bp (delegate Custom|OnPhotonFailed)))

(event Custom|LoadCurrentUserInSpace
  (params (SpaceName :type String))
  (CallFunction|SetCurrentPlayerAvatar)
  (if (Utilities|Enum|Equal(Enum) SpaceName "PersonalSpace")
    (Game|OpenLevel(byName) (Utilities|String|StringToName (Utilities|String|Append "InteriorPreset" (Utilities|String|ToString(Integer) (.currentpersonalspaceid (Variables|Default|GetCurrentLoggedInUser))))))
    (else
      (Game|OpenLevel(byName) (Utilities|String|StringToName SpaceName)))))

(event Custom|InitializeUserPropertyListing
  (Utilities|Array|Add (Variables|Default|GetCTC_CurrentUserPropertyListing) (Utilities|Struct|MakeCTC_UserPropertyListing (Utilities|Struct|MakeCTC_UserData 0 "wajih" "junaid" "wajihjunaid@gmail.com" "wajih" "23") (Utilities|Array|MakeArray (Utilities|Struct|MakeCTC_PropertyData 1 "Map_PS_1" "" "(R=1.000000,G=0.000000,B=0.511661,A=1.000000)" false "1000") (Utilities|Struct|MakeCTC_PropertyData 2 "Map_PS_2" "" "(R=0.056896,G=1.000000,B=0.270162,A=1.000000)" false "2000") (Utilities|Struct|MakeCTC_PropertyData 3 "Map_PS_3" "" "(R=0.000000,G=0.050398,B=1.000000,A=1.000000)" false "3000") (Utilities|Struct|MakeCTC_PropertyData 4 "Map_PS_4" "" "(R=1.000000,G=0.876577,B=0.000000,A=1.000000)" false "4000")))))

(event Custom|SetSelectedPropertiesForSeller
  (params (PropertiesForSeller :type Array%20of%20CTC%20Property%20Data%20Structures))
  (bind _output_get (Variables|CTC_Roles|SetSelectedPropertiesForSeller PropertiesForSeller))
  (for _array_element _output_get
    (Development|PrintString (Utilities|String|Append "Property name: " (.Name (Utilities|Struct|BreakCTC_PropertyData _array_element)) "     " "Updated Price: " (.Price (Utilities|Struct|BreakCTC_PropertyData _array_element))))))

(event Custom|OpenPanel
  (params (PanelToOpen :type User%20Widget%20Class%20Reference) (ClosePrevious? :type Boolean))
  (CallFunction|ClosePanel)
  (if (Utilities|IsValidClass PanelToOpen)
    (Variables|/Script/Engine.PlayerController|SetbShowMouseCursor (Game|GetPlayerController 0) true)
    (bind _returnvalue (UserInterface|CreateWidget PanelToOpen))
    (UserInterface|Viewport|AddtoViewport _returnvalue 0)
    (Variables|Default|SetCurrentOpenedPanel _returnvalue)))

(event Custom|SetSelectedPropertiesForBuyer
  (params (PropertiesForBuyer :type Array%20of%20CTC%20Property%20Data%20Structures))
  (bind _output_get (Variables|CTC_Roles|SetSelectedPropertiesForBuyer PropertiesForBuyer))
  (for _array_element _output_get
    (Development|PrintString (Utilities|String|Append "Property name: " (.Name (Utilities|Struct|BreakCTC_PropertyData _array_element)) "     " "Updated Price: " (.Price (Utilities|Struct|BreakCTC_PropertyData _array_element))))))

(event Custom|SetCurrentPlayerAvatar
  (Variables|Default|SetCurrentSelectedAvatar (.Value (Utilities|Map|Find (Variables|Default|GetAvatarIDs) (.currentselectedavatar (Variables|Default|GetCurrentLoggedInUser))))))

(event Custom|SetSelectedPropertiesForAgent
  (params (PropertiesForAgent :type Array%20of%20CTC%20Agent%20Commision%20Data%20Structures))
  (bind _output_get (Variables|CTC_Roles|SetSelectedPropertiesForAgent PropertiesForAgent))
  (for _array_element _output_get
    (Development|PrintString (Utilities|String|Append "Property name: " (.name (.PropertyData (Utilities|Struct|BreakCTC_AgentCommisionData _array_element))) "     " "Agent comission: " (.AgentCommision (Utilities|Struct|BreakCTC_AgentCommisionData _array_element))))))

(event Custom|ConnectWithPhoton
  (bind _asphoton_cloud_object_api_bp (Utilities|Casting|CastToPhotonCloudObjectAPI_BP (Class|PhotonCloudSubsystem|GetPhotonCloudAPI (Subsystems|GetPhotonCloudSubsystem))))
  (Default|InitGame _asphoton_cloud_object_api_bp (.username (Variables|Default|GetCurrentLoggedInUser)))
  (EventDispatchers|AssignOnPhotonConnectedSuccessfully _asphoton_cloud_object_api_bp (delegate Custom|LoadInDefaultSpace)))