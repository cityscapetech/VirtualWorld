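; BP_ChatHandler connects the virtual world to Photon Chat on BeginPlay and disconnects it on EndPlay.
; Once connected to the chat server, it subscribes to one named channel, printing connection state and subscription results as debug strings.
; Incoming channel and private messages are formatted with the sender's name and broadcast through OnChatMessageRecieved.
; Its send event sends a private message when given a username, otherwise posts to the channel.
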(event Custom|SendMeeage
  (params (Message :type String) (Username :type String))
  (bind _photon_chat_ref (Variables|Default|GetPhoton%20Chat%20Ref))
  (if (> (Utilities|String|Len Username) 0)
    (Class|PhotonChat|SendPrivateMessage _photon_chat_ref Username Message false)
    (else
      (Class|PhotonChat|SendMessage _photon_chat_ref (Variables|Default|GetChatChannelName) Message))))

(event Custom|On%20Photon%20Chat%20Got%20Messages
  (params (ChannelName :type String) (Messages :type Array%20of%20Chat%20Message%20Data%20Structures))
  ;[0.06663 0.1845 0.3185] CHAT
  (Development|PrintString ChannelName)
  (Utilities|Array|Clear (Variables|Default|GetChatMessages))
  (for _array_element Messages
    (Utilities|Array|Add (Variables|Default|GetChatMessages) (Utilities|String|Append "[" (.username _array_element) "]" ":" " " (.message _array_element))))
  (Default|CallOnChatMessageRecieved (Variables|Default|GetChatMessages)))

(event Custom|On%20Photon%20Chat%20new%20State
  (params (State :type EChatConnectionState%20Enum :default "NONE"))
  ;[0.06663 0.1845 0.3185] CHAT
  (Development|PrintString (Utilities|String|Append "CHAT STATE: " (Utilities|String|EnumtoString State)))
  (switch Utilities|FlowControl|Switch|SwitchonEChatConnectionState State
    (:CONNECTED_CHAT
      (Class|PhotonChat|SubscribetoChannels (Variables|Default|GetPhoton%20Chat%20Ref) (Utilities|Array|MakeArray (Variables|Default|GetChatChannelName))))))

(event Custom|OnPhotonChatSubscribeResults%20GO
  (params (ChannelsSubscribeResults :type Array%20of%20Chat%20Subscribe%20Result%20Structures))
  (bind _output (Utilities|Array|Get(acopy) ChannelsSubscribeResults))
  (bind (_name _subscribed) (Utilities|Struct|BreakChatSubscribeResult _output))
  ;[0.06663 0.1845 0.3185] CHAT
  (if (Utilities|Array|IsValidIndex ChannelsSubscribeResults)
    (if _subscribed
      (Development|PrintString (Utilities|String|Append "Joined channel " _name ", sending a message now"))
      (else
        (Development|PrintString "Could not join chat channel" :!label _label)))
    (else
      (goto _label))))

(event Custom|Create%20and%20connect%20Chat
  (bind _photon_chat_ref (Variables|Default|GetPhoton%20Chat%20Ref))
  ;[0.06663 0.1845 0.3185] CHAT
  ;;[1 1 1] Create chat hud
  (EventDispatchers|BindEventtoOnPhotonChatStateChanged _photon_chat_ref (delegate Custom|On%20Photon%20Chat%20new%20State))
  (EventDispatchers|AssignOnPhotonChatSubscribeResults _photon_chat_ref (delegate Custom|OnPhotonChatSubscribeResults%20GO))
  (EventDispatchers|BindEventtoOnPhotonChatGetMessages _photon_chat_ref (delegate Custom|On%20Photon%20Chat%20Got%20Messages))
  (EventDispatchers|AssignOnPhotonChatGetPrivateMessage _photon_chat_ref (delegate Custom|OnPhotonChatGetPrivateMessage_Event))
  (Class|PhotonChat|Connect _photon_chat_ref))

(event Custom|Disconnect%20Chat
  (bind _photon_chat_ref (Variables|Default|GetPhoton%20Chat%20Ref))
  ;[0.06663 0.1845 0.3185] CHAT
  ;;[1 1 1] Create chat hud
  (EventDispatchers|AssignOnPhotonChatStateChanged _photon_chat_ref (delegate Custom|OnPhotonChatStateChanged_Event))
  (Class|PhotonChat|Disconnect _photon_chat_ref))

(event Custom|OnPhotonChatStateChanged_Event
  (params (State :type EChatConnectionState%20Enum :default "NONE"))
  ;[0.06663 0.1845 0.3185] CHAT
  (switch Utilities|FlowControl|Switch|SwitchonEChatConnectionState State
    (:DISCONNECTED
      (Development|PrintString "Chat Disconnected"))))

(event Custom|OnPhotonChatGetPrivateMessage_Event
  (params (UserName :type String) (ChannelName :type String) (Message :type String))
  (bind _chatmessages (Variables|Default|GetChatMessages))
  ;[0.06663 0.1845 0.3185] CHAT
  (Utilities|Array|Clear (Variables|Default|GetChatMessages))
  (Utilities|Array|Add _chatmessages (Utilities|String|Append "[" UserName "]" ":" " " Message))
  (Default|CallOnChatMessageRecieved _chatmessages))

(event EventEndPlay
  (params (EndPlayReason :type EEndPlayReason%20Enum :default "Destroyed"))
  (CallFunction|DisconnectChat))

(event EventBeginPlay
  (Variables|Default|SetPhoton%20Chat%20Ref (Class|PhotonCloudObject|GetPhotonChat (Class|PhotonCloudSubsystem|GetPhotonCloudAPI (Subsystems|GetPhotonCloudSubsystem))))
  (CallFunction|CreateandConnectChat))

(fn ConstructionScript)