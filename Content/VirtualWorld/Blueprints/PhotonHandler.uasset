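; Photon Cloud handler that connects a named player, using that name for all IDs and the password, and manages session events.
; On room join it sets up the local ThirdPersonCharacter, or has the stored player controller spawn a replica for remote players.
; Hit locations and pings go out as player custom properties, but the property-change handler is empty.
; Other callbacks only print status, except disconnect, which also unbinds all events.
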(event Custom|SubscribeEvents
  ;[1 1 1] Subscribe Events
  (Utilities|FlowControl|Sequence
    (:then_0
      (EventDispatchers|AssignOnPhotonCloudConnected (delegate Custom|On%20Connect))
      (EventDispatchers|BindEventtoOnPhotonCloudDisconnected (delegate Custom|OnDisconnected)))
    (:then_1
      (EventDispatchers|BindEventtoOnPlayerJoinedLobbyRoom (delegate Custom|OnPlayerJoinedLobby))
      (EventDispatchers|AssignOnPlayerLeftLobbyRoom (delegate Custom|OnPlayerLeftLobbyRoom_Event)))
    (:then_2
      (EventDispatchers|BindEventtoOnPlayerJoinedRoom (delegate Custom|OnPlayerJoinedGameRoom))
      (EventDispatchers|BindEventtoOnPlayerLeftRoom (delegate Custom|OnPlayerLeftGameRoom)))
    (:then_3
      (EventDispatchers|BindEventtoOnPlayerCustomPropertiesChanged (delegate Custom|OnPlayerPropertiesChanged)))))

(event Custom|On%20Connect
  ;[1 1 1] Subscribe Events
  (Development|PrintString 0 "player connected"))

(event Custom|OnPlayerPropertiesChanged
  (params (PlayerNumber :type Integer) (ChangedProperties :type Photon%20JSON%20Object%20Reference))
  ;[1 1 1] Subscribe Events
)

(event Custom|PingPlayer
  ;[1 1 1] Send Custom Data (avatar, location, color)
  (bind _output_get (Variables|Default|SetData (Class|PhotonJSON|Create self)))
  (bind _returnvalue (Class|PhotonJSON|SetString _output_get "msg"))
  (if (> (Utilities|Array|Length (Class|PhotonJSON|GetObjectKeys _output_get)) 0)
    (Class|PhotonCloudObject|SetPlayerCustomProperties _returnvalue)))

(event Custom|LocationOnHit
  (params (Location :type Vector))
  (bind _output_get (Variables|Default|SetData (Class|PhotonJSON|Create self)))
  (bind _returnvalue (Class|PhotonJSON|SetVector _output_get "Location" Location))
  (Class|PhotonCloudObject|SetPlayerCustomProperties _returnvalue))

(event Custom|ConnectWithPhoton
  (params (PlayerName :type String))
  (CallFunction|SetupIDs PlayerName)
  (CallFunction|SubscribeEvents)
  (Class|PhotonCloudObject|Connect))

(event Custom|OnDisconnected
  ;[1 1 1] Subscribe Events
  (CallFunction|UnSubscribeEvents)
  (Development|PrintString 0 "player disconnected"))

(event Custom|OnPlayerJoinedLobby
  ;[1 1 1] Subscribe Events
  (Development|PrintString 0 "player joined lobby"))

(event Custom|OnPlayerJoinedGameRoom
  (params (PlayerNumber :type Integer) (PlayerName :type String) (IsLocalPlayer :type Boolean))
  (bind _returnvalue (Utilities|Text|ToText(String) PlayerName))
  (bind _playercontrollerref (Variables|Default|GetPlayerControllerRef))
  (bind _returnvalue_2 (Pawn|GetControlledPawn _playercontrollerref))
  (bind _asthird_person_character (Utilities|Casting|CastToThirdPersonCharacter _returnvalue_2))
  ;[1 1 1] Subscribe Events
  (Development|PrintString 0 (Utilities|String|Append "Room joined: \\n" "player number: " (Utilities|String|ToString(Integer) PlayerNumber) "\\n" "Player Name: " PlayerName "\\n" "Is Local Player: " (Utilities|String|ToString(Boolean) IsLocalPlayer)))
  (if (not IsLocalPlayer)
    (bind _replica (Default|CreateCharacterReplica (Variables|Default|GetPlayerControllerRef)))
    (Default|SetupPlayer _replica PlayerNumber self)
    (Default|UpdatePlayerName _replica _returnvalue)
    (else
      (Default|SetupPlayer _asthird_person_character PlayerNumber self)
      (Default|UpdatePlayerName _asthird_person_character _returnvalue))))

(event Custom|OnPlayerLeftLobbyRoom_Event
  ;[1 1 1] Subscribe Events
  (Development|PrintString 0 "player left lobby"))

(event Custom|OnPlayerLeftGameRoom
  (params (PlayerNumber :type Integer))
  ;[1 1 1] Subscribe Events
  (Development|PrintString 0 (Utilities|String|Append "Player left room: " (Utilities|String|ToString(Integer) PlayerNumber))))

(event Custom|UnSubscribeEvents
  ;[1 1 1] UnSubscribe Events
  (Utilities|FlowControl|Sequence
    (:then_0
      (EventDispatchers|UnbindallEventsfromOnPhotonCloudConnected)
      (EventDispatchers|UnbindallEventsfromOnPhotonCloudDisconnected))
    (:then_1
      (EventDispatchers|UnbindallEventsfromOnPlayerJoinedLobbyRoom)
      (EventDispatchers|UnbindallEventsfromOnPlayerLeftLobbyRoom))
    (:then_2
      (EventDispatchers|UnbindallEventsfromOnPlayerJoinedRoom)
      (EventDispatchers|UnbindallEventsfromOnPlayerLeftRoom))
    (:then_3
      (EventDispatchers|UnbindallEventsfromOnPlayerCustomPropertiesChanged))))

(event Custom|SetupIDs
  (params (UID :type String))
  (bind _returnvalue (Class|PhotonCloudObject|GetPhotonCloudConfig))
  ;[1 1 1] Photon IDs Setup
  (Class|PhotonCloudObject|SetPlayerName UID)
  (bind _output_get (Variables|/Script/PhotonCloudAPI.PhotonCloudConfig|SetuserID _returnvalue UID))
  (bind _output_get_2 (Variables|/Script/PhotonCloudAPI.PhotonCloudConfig|SetchatUserID _returnvalue _output_get))
  (bind _output_get_3 (Variables|/Script/PhotonCloudAPI.PhotonCloudConfig|SetuserName _returnvalue _output_get_2))
  (Variables|/Script/PhotonCloudAPI.PhotonCloudConfig|SetuserPassword _returnvalue _output_get_3))

(event EventOnPhotonCloudInitialized
  (Development|PrintString 0 "PhotonInitialized"))

(fn GetPlayerControllerref
  (params (PlayerController :type Player%20Controller%20BP%20Object%20Reference))
  (Variables|Default|SetPlayerControllerRef PlayerController))