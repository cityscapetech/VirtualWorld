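; Short-lived actor that fetches a player's profile by username and spawns their selected avatar in the Photon-networked virtual world.
; On BeginPlay, a VaRest GET request returns user data, whose avatar ID is looked up in the game instance's avatar map.
; The avatar spawns hidden behind a water-ball effect and is revealed after a brief delay.
; It is then set up, named and registered with the Photon player handler before the manager destroys itself.
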(event Custom|OnPlayerDataFetched
  (params (UserData :type CTC%20User%20Data%20Structure))
  (bind _transform (Variables|Default|GetTransform))
  (bind _asgi_virtual_world (Utilities|Casting|CastToGI_VirtualWorld (Game|GetGameInstance)))
  (bind _returnvalue (Game|SpawnActorfromClass (.Value (Utilities|Map|Find (Variables|/Game/VirtualWorld/Blueprints/GI_VirtualWorld.GI_VirtualWorld_C|GetAvatarIDs _asgi_virtual_world) (.currentselectedavatar UserData))) _transform "AlwaysSpawn" 0 0))
  (Rendering|SetActorHiddenInGame _returnvalue true)
  (Game|SpawnActorfromClass "/Game/FXVarietyPack/Blueprints/BP_ky_waterBallHit.BP_ky_waterBallHit_C" _transform "Undefined" 0 0)
  (Utilities|FlowControl|Delay 0.5)
  (Rendering|SetActorHiddenInGame _returnvalue false)
  (Default|SetupPlayer _returnvalue (Variables|Default|GetPlayerNumber) (Variables|Default|GetPhotonCloudRef))
  (Default|UpdatePlayerName _returnvalue (Utilities|Text|ToText(String) (Variables|Default|GetUsername)))
  (bind _outactors (Actor|GetAllActorsOfClass "/Game/VirtualWorld/Blueprints/PhotonClasses/PhotonPlayerHandler_BP.PhotonPlayerHandler_BP_C"))
  (Utilities|Map|Add (Variables|/Game/VirtualWorld/Blueprints/PhotonClasses/PhotonPlayerHandler_BP.PhotonPlayerHandler_BP_C|GetplayerPawns (Utilities|Array|Get(acopy) _outactors)) (Variables|Default|GetPlayerNumber) _returnvalue)
  (Actor|DestroyActor))

(event Custom|OnPlayerDataReceived
  (params (Request :type Va%20Rest%20Request%20JSON%20Object%20Reference))
  (bind _userdata (Default|GetUserData (Variables|Default|GetAPI_Manager) (Class|VaRestJsonObject|GetObjectField (Class|VaRestJsonObject|GetObjectField (Class|VaRestRequestJSON|GetResponseObject Request) "payload") "userData")))
  (CallFunction|OnPlayerDataFetched _userdata))

(event Custom|GetUserDataFromAPI
  (params (Username :type String))
  (Class|VaRestSubsystem|CallURL (|VaRestSubsystem) (Utilities|String|Append (Default|GetAPIFetchPlayerData (Variables|Default|GetAPI_Manager)) "username=" Username) "GET" "json" 0 (delegate Custom|OnPlayerDataReceived)))

(event EventBeginPlay
  (CallFunction|GetUserDatafromAPI (Variables|Default|GetUsername)))

(fn ConstructionScript)