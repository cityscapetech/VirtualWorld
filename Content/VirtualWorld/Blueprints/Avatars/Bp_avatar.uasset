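; Avatar Blueprint for a virtual world that plays looping emotes (clap, wave, thumbs-up, dance) and syncs them over Photon.
; Each local emote event sends an ID through a lazily found PhotonPlayerHandler_BP and toggles that animation on the mesh.
; AnimData mirrors this for a received ID.
; Each emote path has its own FlipFlop, alternating between the clip and returning the mesh to its Animation Blueprint.
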(event Custom|AnimData
  (params (AnimationID :type Integer))
  (bind _mesh (Variables|Character|GetMesh))
  (bind _mesh_2 (Variables|Character|GetMesh))
  (bind _mesh_3 (Variables|Character|GetMesh))
  (bind _mesh_4 (Variables|Character|GetMesh))
  ;[1 1 1] Animation Function
  (CallFunction|InitializeAvatar)
  (switch int AnimationID
    (:1
      (Utilities|FlowControl|FlipFlop
        (:A
          (Components|Animation|PlayAnimation _mesh_3 "/Game/Anim/Clapping_UE_Anim.Clapping_UE_Anim" true))
        (:B
          (Components|Animation|SetAnimationMode _mesh_3 "AnimationBlueprint"))))
    (:2
      (Utilities|FlowControl|FlipFlop
        (:A
          (Components|Animation|PlayAnimation _mesh_4 "/Game/Anim/Waving_Anim.Waving_Anim" true))
        (:B
          (Components|Animation|SetAnimationMode _mesh_4 "AnimationBlueprint"))))
    (:3
      (Utilities|FlowControl|FlipFlop
        (:A
          (Components|Animation|PlayAnimation _mesh "/Game/Anim/ThumbsUp_UE_Anim.ThumbsUp_UE_Anim" true))
        (:B
          (Components|Animation|SetAnimationMode _mesh "AnimationBlueprint"))))
    (:4
      (Utilities|FlowControl|FlipFlop
        (:A
          (Components|Animation|PlayAnimation _mesh_2 "/Game/Anim/Dancing_UE_Anim.Dancing_UE_Anim" true))
        (:B
          (Components|Animation|SetAnimationMode _mesh_2 "AnimationBlueprint"))))))

(event Custom|DanceAnim
  (bind _mesh (Variables|Character|GetMesh))
  ;[1 1 1] Custom Animation
  (CallFunction|InitializeAvatar)
  (Default|SendAnimData (Variables|Default|GetPhotonHandler) 4)
  (Utilities|FlowControl|FlipFlop
    (:A
      (Components|Animation|PlayAnimation _mesh "/Game/Anim/Dancing_UE_Anim.Dancing_UE_Anim" true))
    (:B
      (Components|Animation|SetAnimationMode _mesh "AnimationBlueprint"))))

(event Custom|CallAnim
  (bind _mesh (Variables|Character|GetMesh))
  ;[1 1 1] Custom Animation
  (CallFunction|InitializeAvatar)
  (Default|SendAnimData (Variables|Default|GetPhotonHandler) 1)
  (Utilities|FlowControl|FlipFlop
    (:A
      (Components|Animation|PlayAnimation _mesh "/Game/Anim/Clapping_UE_Anim.Clapping_UE_Anim" true))
    (:B
      (Components|Animation|SetAnimationMode _mesh "AnimationBlueprint"))))

(event Custom|InitializeAvatar
  (Utilities|IsValid (Variables|Default|GetPhotonHandler)
    (:Is%20Not%20Valid
      (bind _outactors (Actor|GetAllActorsOfClass "/Game/VirtualWorld/Blueprints/PhotonClasses/PhotonPlayerHandler_BP.PhotonPlayerHandler_BP_C"))
      (Variables|Default|SetPhotonHandler (Utilities|Array|Get(acopy) _outactors)))))

(event Custom|WaveAnim
  (bind _mesh (Variables|Character|GetMesh))
  ;[1 1 1] Custom Animation
  (CallFunction|InitializeAvatar)
  (Default|SendAnimData (Variables|Default|GetPhotonHandler) 2)
  (Utilities|FlowControl|FlipFlop
    (:A
      (Components|Animation|PlayAnimation _mesh "/Game/Anim/Waving_Anim.Waving_Anim" true))
    (:B
      (Components|Animation|SetAnimationMode _mesh "AnimationBlueprint"))))

(event Custom|ThanksAnim
  (bind _mesh (Variables|Character|GetMesh))
  ;[1 1 1] Custom Animation
  (CallFunction|InitializeAvatar)
  (Default|SendAnimData (Variables|Default|GetPhotonHandler) 3)
  (Utilities|FlowControl|FlipFlop
    (:A
      (Components|Animation|PlayAnimation _mesh "/Game/Anim/ThumbsUp_UE_Anim.ThumbsUp_UE_Anim" true))
    (:B
      (Components|Animation|SetAnimationMode _mesh "AnimationBlueprint"))))

(fn ConstructionScript)