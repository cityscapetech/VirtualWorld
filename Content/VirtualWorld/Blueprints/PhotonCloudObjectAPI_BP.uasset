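; Photon Cloud API Blueprint that manages the game's connection session and re-broadcasts connection success or failure.
; InitGame runs once until reset: it caches the user name, copies it into every Photon config credential field including password, binds callbacks, then connects.
; Errors notify listeners and print for selected codes; state changes are only printed.
; A controller-ready event caches the local controller and its player starts.
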(event Custom|InitGame
  (params (UserName :type String))
  ;[1 1 1] cache
  (if (not (Variables|Default|GetbGameInitialized))
    (Variables|Default|SetCurrentPlayerUserName UserName)
    (CallFunction|SubscribePhotonEvents)
    (Variables|Default|SetbGameInitialized true)
    ;[1 1 1] Connect
    (EventDispatchers|AssignOnPhotonCloudConnected (delegate Custom|On%20Connect))
    (Class|PhotonCloudObject|SetPlayerName (Variables|Default|GetCurrentPlayerUserName))
    (Class|PhotonCloudObject|Connect)))

(event Custom|On%20Connect
  ;[1 1 1] Connect
  (Development|PrintString 0 "Photon connected successfully")
  (Default|CallOnPhotonConnectedSuccessfully))

(event Custom|On%20Photon%20Connection%20Error
  (params (ErrorCode :type EPhotonErrorCode%20Enum :default "OK") (ErrorMessage :type String))
  ;[1 1 1] ON DISCONNECTION
  (Default|CallOnPhotonConnectionFailed)
  (switch Utilities|FlowControl|Switch|SwitchonEPhotonErrorCode ErrorCode
    (:OPERATION_DENIED
      _)
    (:OPERATION_INVALID
      _)
    (:INTERNAL_SERVER_ERROR
      _)
    (:INVALID_AUTHENTICATION
      _)
    (:SERVER_FULL
      _)
    (:USER_BLOCKED
      _)
    (:INVALID_REGION
      _))
  (Development|PrintString self ErrorMessage))

(event Custom|ResetPhotonSession
  (Variables|Default|SetLocalController 0)
  (Variables|Default|SetbGameInitialized false)
  (Variables|Default|SetCurrentPlayerUserName ""))

(event Custom|On%20Controller%20Is%20Ready
  (params (3rd%20Player%20Controler%20 :type Player%20Controller%20BP%20Object%20Reference))
  (Variables|Default|SetLocalController 3rd%20Player%20Controler%20)
  (Variables|Default|SetPlayerStarts (Default|GetPlayerStarts (Variables|Default|GetLocalController))))

(event Custom|On%20Photon%20Cloud%20Event%20Changed
  (params (NewState :type EPhotonCloudStates%20Enum :default "UNINITIALIZED"))
  ;[1 1 1] PHOTON CLOUD STATE CHANGED
  (Development|PrintString self (Utilities|String|EnumtoString NewState) true true "(R=0.214249,G=0.326103,B=1.000000,A=1.000000)" 3.0)
  (switch Utilities|FlowControl|Switch|SwitchonEPhotonCloudStates NewState))

(event Custom|SubscribePhotonEvents
  (bind _returnvalue (Class|PhotonCloudObject|GetPhotonCloudConfig))
  (Utilities|FlowControl|Sequence
    (:then_0
      ;[1 1 1] ON DISCONNECTION
      (EventDispatchers|AssignOnPhotonConnectionError (delegate Custom|On%20Photon%20Connection%20Error)))
    (:then_1
      ;[1 1 1] PHOTON CLOUD STATE CHANGED
      (EventDispatchers|AssignOnPhotonCloudStateChanged (delegate Custom|On%20Photon%20Cloud%20Event%20Changed))
      (bind _output_get (Variables|/Script/PhotonCloudAPI.PhotonCloudConfig|SetuserID _returnvalue (Variables|Default|GetCurrentPlayerUserName)))
      (bind _output_get_2 (Variables|/Script/PhotonCloudAPI.PhotonCloudConfig|SetchatUserID _returnvalue _output_get))
      (bind _output_get_3 (Variables|/Script/PhotonCloudAPI.PhotonCloudConfig|SetuserName _returnvalue _output_get_2))
      (Variables|/Script/PhotonCloudAPI.PhotonCloudConfig|SetuserPassword _returnvalue _output_get_3))))