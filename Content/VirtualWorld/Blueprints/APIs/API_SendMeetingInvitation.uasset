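; One-shot API actor that sends a meeting invitation to the backend for the virtual world.
; SendMeetingInvitation passes the invite's ID, title, organizer and receiver as query parameters in a VaRest GET call.
; The response callback prints each returned meeting title, fires OnInvitationSentSuccessfully without checking for failure, then destroys the actor.
; A GetUserData helper, unused here, converts user JSON into CTCUserData with a role enum.
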(event Custom|SendMeetingInvitation
  (params (MeetingInvite :type CTC%20Meeting%20Invitation%20Structure))
  (bind (_meetingid _meetingtitle _organizer _receiver) (Utilities|Struct|BreakCTC_MeetingInvitation MeetingInvite))
  (Class|VaRestSubsystem|CallURL (|VaRestSubsystem) (Utilities|String|Append (Variables|APIs|GetAPI_SendMeetingInvite) "meetingID=" _meetingid "&meetingTitle=" _meetingtitle "&organizer=" _organizer "&receiver=" _receiver) "GET" "json" 0 (delegate Custom|OnMeetingSendResponseReceived)))

(event Custom|OnMeetingSendResponseReceived
  (params (Request :type Va%20Rest%20Request%20JSON%20Object%20Reference))
  (for _array_element (Class|VaRestJsonValue|AsArray (Class|VaRestRequestJSON|GetResponseValue Request))
    (bind _returnvalue (Class|VaRestJsonValue|AsObject _array_element))
    (Development|PrintString (Utilities|String|Append (Class|VaRestJsonObject|GetStringField _returnvalue "meetingTitle") " invitation sent to: " (.Receiver (Utilities|Struct|BreakCTC_MeetingInvitation (stale Custom|SendMeetingInvitation MeetingInvite))))))
  (Default|CallOnInvitationSentSuccessfully)
  (Actor|DestroyActor))

(fn ConstructionScript)

(fn GetUserData
  (params (JsonObj :type Va%20Rest%20Json%20Object%20Object%20Reference))
  (Utilities|FlowControl|Sequence
    (:then_0
      (switch string (Class|VaRestJsonObject|GetStringField JsonObj "role")
        (:agent
          (LocalVariables|SetCurrentRole "NewEnumerator0"))
        (:buyer
          (LocalVariables|SetCurrentRole "NewEnumerator2"))
        (:seller
          (LocalVariables|SetCurrentRole "NewEnumerator1"))
        (:guest
          (LocalVariables|SetCurrentRole "NewEnumerator3"))))
    (:then_1
      (return (Utilities|Struct|MakeCTC_UserData 0 (Class|VaRestJsonObject|GetStringField JsonObj "firstName") (Class|VaRestJsonObject|GetStringField JsonObj "lastName") "" (Class|VaRestJsonObject|GetStringField JsonObj "username") (Class|VaRestJsonObject|GetStringField JsonObj "password") "" (Math|Conversions|ToInteger(Byte) (Class|VaRestJsonObject|GetStringField JsonObj "personalSpaceID")) (Class|VaRestJsonObject|GetStringField JsonObj "avatarID") (LocalVariables|GetCurrentRole))))))