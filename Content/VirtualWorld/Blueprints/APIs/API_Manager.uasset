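; API manager actor for the virtual world that handles login, signup, user lookup, user lists and meeting invitations against a backend.
; VaRest sends GET requests with query-string parameters, passwords included, to a domain switchable to local.
; JSON callbacks broadcast results, store the logged-in user in GI_VirtualWorld, or push lists to a Context object.
; Sending an invite uses a spawned API actor and hardcoded meeting details, then opens MeetingRoomMap on success.
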(event Custom|FetchInvitations
  (params (username :type String) (Context :type W%20Received%20Invitation%20List%20Object%20Reference))
  (Class|VaRestSubsystem|CallURL (|VaRestSubsystem) (Utilities|String|Append (Utilities|String|Append (Variables|APIs|GetFinalDomain) (Variables|APIs|GetAPI_FetchAllInvitations)) "receiver=" username) "GET" "json" 0 (delegate Custom|OnInvitationsFetched)))

(event Custom|OnInvitationsFetched
  (params (Request :type Va%20Rest%20Request%20JSON%20Object%20Reference))
  (Utilities|Array|Clear (Variables|Default|GetMeetingInvitations))
  (for _array_element (Class|VaRestJsonValue|AsArray (Class|VaRestRequestJSON|GetResponseValue Request))
    (bind _returnvalue (Class|VaRestJsonValue|AsObject _array_element))
    (Utilities|Array|Add (Variables|Default|GetMeetingInvitations) (Utilities|Struct|MakeCTC_MeetingInvitation "" (Class|VaRestJsonObject|GetStringField _returnvalue "meetingTitle") (Class|VaRestJsonObject|GetStringField _returnvalue "organizer") "")))
  (Default|SetData (stale Custom|FetchInvitations Context) (Variables|Default|GetMeetingInvitations)))

(event Custom|OnFindUserDataResponseReceived
  (params (Request :type Va%20Rest%20Request%20JSON%20Object%20Reference))
  (bind _returnvalue (Class|VaRestJsonValue|AsObject (Class|VaRestRequestJSON|GetResponseValue Request)))
  (if (== (Class|VaRestJsonObject|GetIntegerField (Class|VaRestJsonObject|GetObjectField _returnvalue "payload") "resultCode") 200)
    (Default|CallOnFetchUserDataResponse true)
    (else
      (Default|CallOnFetchUserDataResponse false))))

(event Custom|OnInvitationSent
  (bind _gameinstancevw (Variables|Default|GetGameInstanceVW))
  ;[1 1 1] SendMeetingInvitation
  (Variables|/Game/VirtualWorld/Blueprints/GI_VirtualWorld.GI_VirtualWorld_C|SetCurrentJoinedMeetingData _gameinstancevw (Variables|Default|GetMeetingInvite))
  (Default|OpenPanel _gameinstancevw "/Game/VirtualWorld/Blueprints/Widgets/AccountDetails/InGameWidgets/MeetingRoom/W_ConnectingToMeeting.W_ConnectingToMeeting_C" true)
  (Utilities|FlowControl|Delay 2.0)
  (Game|OpenLevel(byName) "MeetingRoomMap"))

(event Custom|GetAllUsers
  (params (Context :type W%20Send%20Invite%20List%20Object%20Reference))
  (Utilities|Array|Clear (Variables|Default|GetUsers))
  (Class|VaRestSubsystem|CallURL (|VaRestSubsystem) (Utilities|String|Append (Variables|APIs|GetFinalDomain) (Variables|APIs|GetAPI_FetchAllUsers)) "GET" "json" 0 (delegate Custom|OnAllUsersReceived)))

(event Custom|OnAllUsersReceived
  (params (Request :type Va%20Rest%20Request%20JSON%20Object%20Reference))
  (for _array_element (Class|VaRestJsonValue|AsArray (Class|VaRestRequestJSON|GetResponseValue Request))
    (bind _returnvalue (Class|VaRestJsonValue|AsObject _array_element))
    (bind _userdata (CallFunction|GetUserData _returnvalue))
    (Utilities|Array|Add (Variables|Default|GetUsers) _userdata))
  (Default|SetData (stale Custom|GetAllUsers Context) (Variables|Default|GetUsers)))

(event Custom|Signup
  (bind _gameinstancevw (Variables|Default|GetGameInstanceVW))
  (bind _currentloggedinuser (Variables|/Game/VirtualWorld/Blueprints/GI_VirtualWorld.GI_VirtualWorld_C|GetCurrentLoggedInUser _gameinstancevw))
  (Class|VaRestSubsystem|CallURL (|VaRestSubsystem) (Utilities|String|Append (Utilities|String|Append (Variables|APIs|GetFinalDomain) (Variables|APIs|GetAPI_Signup)) "username=" (.username _currentloggedinuser) "&password=" (.password _currentloggedinuser) "&role=" (Utilities|String|EnumtoString (.userrole _currentloggedinuser)) "&gender=" (.gender _currentloggedinuser) "&personalSpaceID=" (Utilities|String|ToString(Integer) (.currentpersonalspaceid _currentloggedinuser)) "&avatarID=" (.currentselectedavatar _currentloggedinuser)) "GET" "json" 0 (delegate Custom|SignupResponseReceived)))

(event Custom|Login
  (params (username :type String) (password :type String))
  (bind _asgi_virtual_world (Utilities|Casting|CastToGI_VirtualWorld (Game|GetGameInstance)))
  (Variables|/Game/VirtualWorld/Blueprints/GI_VirtualWorld.GI_VirtualWorld_C|SetCurrentLoggedInUser _asgi_virtual_world (Utilities|Struct|MakeCTC_UserData 0 "" "" "" username password "" 0 "" "NewEnumerator0" false))
  (Class|VaRestSubsystem|CallURL (|VaRestSubsystem) (Utilities|String|Append (Utilities|String|Append (Variables|APIs|GetFinalDomain) (Variables|APIs|GetAPI_Login)) "username=" username "&password=" password) "GET" "json" 0 (delegate Custom|LoginResponse)))

(event Custom|LoginResponse
  (params (Request :type Va%20Rest%20Request%20JSON%20Object%20Reference))
  (bind _returnvalue (Class|VaRestJsonValue|AsObject (Class|VaRestRequestJSON|GetResponseValue Request)))
  (Utilities|IsValid _returnvalue
    (:Is%20Valid
      (if (== (Class|VaRestJsonObject|GetIntegerField (Class|VaRestJsonObject|GetObjectField _returnvalue "payload") "resultCode") 200)
        (Default|CallOnLoginResponse true (Class|VaRestJsonObject|GetStringField (Class|VaRestJsonObject|GetObjectField _returnvalue "payload") "message"))
        (bind _userdata (CallFunction|GetUserData (Class|VaRestJsonObject|GetObjectField (Class|VaRestJsonObject|GetObjectField _returnvalue "payload") "userData")))
        (bind _asgi_virtual_world (Utilities|Casting|CastToGI_VirtualWorld (Game|GetGameInstance)))
        (Variables|/Game/VirtualWorld/Blueprints/GI_VirtualWorld.GI_VirtualWorld_C|SetCurrentLoggedInUser _asgi_virtual_world _userdata)
        (else
          (Default|CallOnLoginResponse false (Class|VaRestJsonObject|GetStringField (Class|VaRestJsonObject|GetObjectField _returnvalue "payload") "message")))))
    (:Is%20Not%20Valid
      (Default|CallOnLoginResponse false "Failed to login to server, please try again"))))

(event Custom|SignupResponseReceived
  (params (Request :type Va%20Rest%20Request%20JSON%20Object%20Reference))
  (bind _returnvalue (Class|VaRestJsonValue|AsObject (Class|VaRestRequestJSON|GetResponseValue Request)))
  (if (== (Class|VaRestJsonObject|GetIntegerField (Class|VaRestJsonObject|GetObjectField _returnvalue "payload") "resultCode") 200)
    (Default|CallOnSignupResponse true (Class|VaRestJsonObject|GetStringField (Class|VaRestJsonObject|GetObjectField _returnvalue "payload") "message"))
    (else
      (Default|CallOnSignupResponse false (Class|VaRestJsonObject|GetStringField (Class|VaRestJsonObject|GetObjectField _returnvalue "payload") "message")))))

(event Custom|SendMeetingInvitation
  (params (Receiver :type String))
  ;[1 1 1] SendMeetingInvitation
  (Default|OpenPanel (Variables|Default|GetGameInstanceVW) "/Game/VirtualWorld/Blueprints/Widgets/AccountDetails/InGameWidgets/MeetingRoom/W_SendingMeetingInvite.W_SendingMeetingInvite_C" true)
  (Utilities|FlowControl|Delay 2.0)
  (bind _output_get (Variables|Default|SetMeetingInvite (Utilities|Struct|MakeCTC_MeetingInvitation "123" "WajihMeeting" (.username (Variables|/Game/VirtualWorld/Blueprints/GI_VirtualWorld.GI_VirtualWorld_C|GetCurrentLoggedInUser (Variables|Default|GetGameInstanceVW))) Receiver)))
  (bind _returnvalue (Game|SpawnActorfromClass "/Game/VirtualWorld/Blueprints/APIs/API_SendMeetingInvitation.API_SendMeetingInvitation_C" (Math|Transform|MakeTransform "0, 0, 0" "0, 0, 0" "1.000000,1.000000,1.000000") "Undefined" 0 0))
  (Default|SendMeetingInvitation _returnvalue _output_get)
  (EventDispatchers|BindEventtoOnInvitationSentSuccessfully _returnvalue (delegate Custom|OnInvitationSent)))

(event Custom|Relog%20in
  (bind _asgi_virtual_world (Utilities|Casting|CastToGI_VirtualWorld (Game|GetGameInstance)))
  (CallFunction|Login (.username (Variables|/Game/VirtualWorld/Blueprints/GI_VirtualWorld.GI_VirtualWorld_C|GetCurrentLoggedInUser _asgi_virtual_world)) (.password (Variables|/Game/VirtualWorld/Blueprints/GI_VirtualWorld.GI_VirtualWorld_C|GetCurrentLoggedInUser _asgi_virtual_world))))

(event Custom|CheckIfUserExists
  (params (username :type String))
  (Class|VaRestSubsystem|CallURL (|VaRestSubsystem) (Utilities|String|Append (Utilities|String|Append (Variables|APIs|GetFinalDomain) (Variables|APIs|GetAPI_FindUser)) "username=" username) "GET" "json" 0 (delegate Custom|OnFindUserDataResponseReceived)))

(event EventBeginPlay
  (bind _asgi_virtual_world (Utilities|Casting|CastToGI_VirtualWorld (Game|GetGameInstance)))
  (Variables|Default|SetGameInstanceVW _asgi_virtual_world)
  (if (Variables|Default|GetisDeployedLocal?)
    (Variables|APIs|SetFinalDomain (Variables|APIs|GetDomainLocal))))

(fn ConstructionScript)

(fn GetUserData
  (params (JsonObj :type Va%20Rest%20Json%20Object%20Object%20Reference))
  (Utilities|FlowControl|Sequence
    (:then_0
      (switch string (Class|VaRestJsonObject|GetStringField JsonObj "role")
        (:agent
          (LocalVariables|SetCurrentRole "NewEnumerator0"))
        (:buyer
          (LocalVariables|SetCurrentRole "NewEnumerator2"))
        (:seller
          (LocalVariables|SetCurrentRole "NewEnumerator1"))
        (:guest
          (LocalVariables|SetCurrentRole "NewEnumerator3"))))
    (:then_1
      (return (Utilities|Struct|MakeCTC_UserData 0 (Class|VaRestJsonObject|GetStringField JsonObj "firstName") (Class|VaRestJsonObject|GetStringField JsonObj "lastName") "" (Class|VaRestJsonObject|GetStringField JsonObj "username") (Class|VaRestJsonObject|GetStringField JsonObj "password") "" (Math|Conversions|ToInteger(Byte) (Class|VaRestJsonObject|GetStringField JsonObj "personalSpaceID")) (Class|VaRestJsonObject|GetStringField JsonObj "avatarID") (LocalVariables|GetCurrentRole))))))

(fn GetAPIFetchPlayerData
  (return (Utilities|String|Append (Variables|APIs|GetFinalDomain) (Variables|APIs|GetAPI_FetchPlayerData))))