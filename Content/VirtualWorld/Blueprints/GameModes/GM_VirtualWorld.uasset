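; Game mode for the virtual world that swaps the player's pawn for the avatar selected in the game instance.
; On BeginPlay it opens the environment loading panel, sets the default pawn class to that avatar, and destroys the existing pawn.
; It then spawns and possesses the avatar at the player start, keeping it hidden until a delayed water-ball hit actor spawns there, then reveals it shortly after.
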(event Custom|SetPawn
  (bind _returnvalue (Game|GetPlayerController 0))
  (bind _returnvalue_2 (Class|GameModeBase|FindPlayerStart _returnvalue))
  (bind _returnvalue_3 (Transformation|GetActorLocation _returnvalue_2))
  (bind _returnvalue_4 (Game|SpawnActorfromClass (Variables|Default|GetDefaultPawnClass) (Math|Transform|MakeTransform _returnvalue_3 (Transformation|GetActorRotation _returnvalue_2) "1.000000,1.000000,1.000000") "Undefined" 0 0))
  (Pawn|Possess (Game|GetPlayerController 0) _returnvalue_4)
  (Rendering|SetActorHiddenInGame _returnvalue_4 true)
  (Utilities|FlowControl|Delay 2.0)
  (Game|SpawnActorfromClass "/Game/FXVarietyPack/Blueprints/BP_ky_waterBallHit.BP_ky_waterBallHit_C" (Math|Transform|MakeTransform _returnvalue_3 "0, 0, 0" "1.000000,1.000000,1.000000") "Undefined" 0 0)
  (Utilities|FlowControl|Delay 0.5)
  (Rendering|SetActorHiddenInGame _returnvalue_4 false))

(event Custom|DestroyOldPawn
  (bind _returnvalue (Game|Player|GetPlayerPawn 0))
  (Utilities|IsValid _returnvalue
    (:Is%20Valid
      (Actor|DestroyActor _returnvalue))))

(event EventBeginPlay
  (bind _asgi_virtual_world (Utilities|Casting|CastToGI_VirtualWorld (Game|GetGameInstance)))
  (Utilities|FlowControl|Sequence
    (:then_0
      (Default|OpenPanel _asgi_virtual_world "/Game/VirtualWorld/Blueprints/Widgets/UserCredentials/W_LoadingEnviroment.W_LoadingEnviroment_C" true))
    (:then_1
      (Variables|Default|SetDefaultPawnClass (Variables|/Game/VirtualWorld/Blueprints/GI_VirtualWorld.GI_VirtualWorld_C|GetCurrentSelectedAvatar _asgi_virtual_world)))
    (:then_2
      (CallFunction|DestroyOldPawn))
    (:then_3
      (CallFunction|SetPawn))))

(fn ConstructionScript)