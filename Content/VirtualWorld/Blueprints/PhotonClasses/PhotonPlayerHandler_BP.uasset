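; Photon multiplayer player handler that tracks room members' pawns by player number and relays their animation IDs.
; Binds Photon join, leave and data events, setting up the local character or requesting replicas at random player starts.
; Animation IDs travel as JSON to each Bp_avatar.
; Leaving players' pawns are destroyed; local departure clears all and calls JoinRoomIfNeeded, an empty event here that JoinRoom also uses when roomless.
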(event Custom|OnPlayerJoined
  (params (PlayerNumber :type Integer) (PlayerName :type String) (IsLocalPlayer :type Boolean))
  ;[1 1 1] Binding On Player Joined Room Event
  (CallFunction|OnThirdPersonJoined PlayerNumber PlayerName IsLocalPlayer)
  (bind _asgi_virtual_world (Utilities|Casting|CastToGI_VirtualWorld (Game|GetGameInstance)))
  (Default|OpenPanel _asgi_virtual_world "/Game/VirtualWorld/Blueprints/Widgets/AccountDetails/InGameWidgets/W_UserProfileMain.W_UserProfileMain_C" true))

(event Custom|OnPlayerLeftRoom
  (params (PlayerNumber :type Integer))
  (bind _playerpawns (Variables|Default|GetplayerPawns))
  (bind (_value _returnvalue) (Utilities|Map|Find _playerpawns PlayerNumber))
  ;[1 1 1] Binding On Player Left Room Event
  (if _returnvalue
    (Utilities|FlowControl|Sequence
      (:then_0
        (Utilities|IsValid _value
          (:Is%20Valid
            (Actor|DestroyActor _value))))
      (:then_1
        (if (== PlayerNumber (Variables|Default|GetlocalPlayerPhotonID))
          (CallFunction|ClearAllPlayers)
          (CallFunction|JoinRoomifNeeded))))
    (elif (== (Utilities|Map|Length _playerpawns) 0)
      (CallFunction|JoinRoomifNeeded))))

(event Custom|SendAnimData
  (params (AnimID :type Integer))
  ;[1 1 1] SendPlayerData
  (bind _returnvalue (Class|PhotonJSON|SetInteger (Class|PhotonJSON|Create self) "AnimData" AnimID))
  (Class|PhotonCloudObject|SendPlayerData (Variables|Default|GetphotonCloudObjectReference) _returnvalue 0 "DO_NOT_CACHE" true 0 "OTHERS"))

(event Custom|OnThirdPersonJoined
  (params (playerNumber :type Integer) (playerName :type String) (isLocalPlayer :type Boolean))
  (bind _photoncloudobjectreference (Variables|Default|GetphotonCloudObjectReference))
  (bind _photoncloudobjectreference_2 (Variables|Default|GetphotonCloudObjectReference))
  (bind _photoncloudobjectreference_3 (Variables|Default|GetphotonCloudObjectReference))
  (bind _localcontroller (Variables|/Game/VirtualWorld/Blueprints/PhotonCloudObjectAPI_BP.PhotonCloudObjectAPI_BP_C|GetLocalController _photoncloudobjectreference))
  (bind _playerstarts (Variables|/Game/VirtualWorld/Blueprints/PhotonCloudObjectAPI_BP.PhotonCloudObjectAPI_BP_C|GetPlayerStarts _photoncloudobjectreference_2))
  (bind _returnvalue (Utilities|Array|Length _playerstarts))
  (bind _returnvalue_2 (Pawn|GetControlledPawn _localcontroller))
  (bind _returnvalue_3 (- _returnvalue 1))
  (bind _asthird_person_character (Utilities|Casting|CastToThirdPersonCharacter _returnvalue_2))
  (bind _returnvalue_4 (Math|Random|RandomIntegerinRange 0 _returnvalue_3))
  (bind _output (Utilities|Array|Get(acopy) _playerstarts _returnvalue_4))
  (bind _returnvalue_5 (Transformation|GetActorTransform _output))
  ;[1 1 1] OnThird Person Joined Event
  (if (not (Utilities|Map|Contains (Variables|Default|GetplayerPawns) playerNumber))
    (if isLocalPlayer
      (Variables|Default|SetlocalPlayerPhotonID playerNumber)
      (Default|SetupPlayer _asthird_person_character playerNumber (Variables|Default|GetphotonCloudObjectReference))
      (Utilities|Map|Add (Variables|Default|GetplayerPawns) playerNumber _asthird_person_character)
      (Default|UpdatePlayerName _asthird_person_character (Utilities|Text|ToText(String) playerName))
      (else
        (Default|FetchandCreatePlayerReplica (Variables|/Game/VirtualWorld/Blueprints/PhotonCloudObjectAPI_BP.PhotonCloudObjectAPI_BP_C|GetLocalController _photoncloudobjectreference_3) playerName playerNumber _photoncloudobjectreference_3 (Math|Transform|MakeTransform (.location _returnvalue_5) (.rotation _returnvalue_5)))))))

(event Custom|Subscribe%20Event
  ;[1 1 1] Getting Photon Cloud Class Refernce
  (bind _asphoton_cloud_object_api_bp (Utilities|Casting|CastToPhotonCloudObjectAPI_BP (Class|PhotonCloudSubsystem|GetPhotonCloudAPI (Subsystems|GetPhotonCloudSubsystem))))
  (Variables|Default|SetphotonCloudObjectReference _asphoton_cloud_object_api_bp)
  (Utilities|FlowControl|Sequence
    (:then_0
      ;[1 1 1] Binding On Player Joined Room Event
      (EventDispatchers|BindEventtoOnPlayerJoinedRoom (Variables|Default|GetphotonCloudObjectReference) (delegate Custom|OnPlayerJoined)))
    (:then_1
      ;[1 1 1] Binding On Player Left Room Event
      (EventDispatchers|BindEventtoOnPlayerLeftRoom (Variables|Default|GetphotonCloudObjectReference) (delegate Custom|OnPlayerLeftRoom)))
    (:then_2
      ;[1 1 1] Receive Player Data
      (EventDispatchers|BindEventtoOnReceivedPlayerData (Variables|Default|GetphotonCloudObjectReference) (delegate Custom|ReceivedPlayerData)))))

(event Custom|ClearAllPlayers
  (bind _playerpawns (Variables|Default|GetplayerPawns))
  ;[1 1 1] Clear Players Event
  (bind _keys (Utilities|Map|Keys _playerpawns))
  (for _array_element _keys
    (Utilities|IsValid (.Value (Utilities|Map|Find _playerpawns _array_element))
      (:Is%20Valid
        (Actor|DestroyActor (.Value (Utilities|Map|Find _playerpawns _array_element))))))
  (Utilities|Map|Clear (Variables|Default|GetplayerPawns)))

(event Custom|JoinRoomIfNeeded)

(event Custom|ReceivedPlayerData
  (params (PlayerNumber :type Integer) (DataJSON :type Photon%20JSON%20Object%20Reference))
  ;[1 1 1] Receive Player Data
  (bind _asbp_avatar (Utilities|Casting|CastToBp_avatar (.Value (Utilities|Map|Find (Variables|Default|GetplayerPawns) PlayerNumber))))
  (Default|AnimData _asbp_avatar (Class|PhotonJSON|GetInteger DataJSON "AnimData")))

(event Collision|EventActorBeginOverlap
  (params (OtherActor :type Actor%20Object%20Reference)))

(event EventTick
  (params (DeltaSeconds :type Float%20%28single-precision%29)))

(event EventEndPlay
  (params (EndPlayReason :type EEndPlayReason%20Enum :default "Destroyed"))
  (bind _photoncloudobjectreference (Variables|Default|GetphotonCloudObjectReference))
  ;[1 1 1] OnDestroy Event
  (Utilities|FlowControl|Sequence
    (:then_0
      (EventDispatchers|UnbindallEventsfromOnPlayerJoinedRoom _photoncloudobjectreference))
    (:then_1
      (EventDispatchers|UnbindallEventsfromOnPlayerLeftRoom _photoncloudobjectreference))
    (:then_2
      (EventDispatchers|UnbindallEventsfromOnReceivedPlayerData _photoncloudobjectreference))))

(fn ConstructionScript)

(fn JoinRoom
  (params (roomName :type String))
  (Variables|Default|SetRoomName roomName)
  (if (Utilities|Array|IsEmpty (Class|PhotonCloudObject|GetRoomName (Variables|Default|GetphotonCloudObjectReference)))
    (CallFunction|JoinRoomifNeeded)
    (else
      (Class|PhotonCloudObject|LeaveRoom (Variables|Default|GetphotonCloudObjectReference) false false))))