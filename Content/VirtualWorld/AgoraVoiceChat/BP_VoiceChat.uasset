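; Voice chat Blueprint that joins an Agora RTC channel on BeginPlay, publishing the microphone and auto-subscribing to audio only.
; It requests Android permissions, spawns the engine and event handler actors, then binds join, leave and offline callbacks.
; Callbacks mostly print status, though join success and user offline also make video canvas setup calls.
; EndPlay releases the engine, and separate functions leave the channel or return to the main level.
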(event EventBeginPlay
  (CallFunction|CheckPermission)
  (Variables|/Script/Engine.PlayerController|SetbShowMouseCursor (Game|GetPlayerController 0) true)
  (CallFunction|InitRtcEngine)
  (CallFunction|JoinChannelClick))

(event EventEndPlay
  (params (EndPlayReason :type EEndPlayReason%20Enum :default "Destroyed"))
  (Class|AgoraRtcEngine|Release (Variables|Default|GetRtcEngine) false)
  (Actor|DestroyActor (Variables|Default|GetEventHandler)))

(fn ConstructionScript)

(fn JoinChannelClick
  (Class|AgoraRtcEngine|EnableAudio (Variables|Default|GetRtcEngine))
  (|SetBy-RefVar (stale _options) (Utilities|Struct|MakeChannelMediaOptions "AGORA_FALSE_VALUE" "AGORA_TRUE_VALUE" "AGORA_FALSE_VALUE" "AGORA_FALSE_VALUE" "AGORA_FALSE_VALUE" "AGORA_TRUE_VALUE" "AGORA_FALSE_VALUE" "AGORA_TRUE_VALUE" "AGORA_TRUE_VALUE"))
  (bind _options (Class|AgoraRtcEngine|JoinChannel (Variables|Default|GetRtcEngine) (Variables|Default|GetToken) (Variables|Default|GetChannelId))))

(fn LeaveChannelClick
  (Class|AgoraRtcEngine|LeaveChannel (Variables|Default|GetRtcEngine))
  (Viewport|RemoveAllWidgets))

(fn OnUserJoinCallBack
  (params (Uid :type Integer64) (Elapsed :type Integer))
  (Development|PrintString (Utilities|String|Append "user join uid is" (Utilities|String|ToString(Integer) Elapsed))))

(fn OnUserJoinChannelSuccess
  (params (Channel :type String) (Uid :type Integer64) (Elapsed :type Integer))
  (Development|PrintString (Utilities|String|Append "joinchannel succees ChannelName is " Channel ",uid is " (Utilities|String|ToString(Text) (Utilities|Text|ToText(String) Uid)) "elapse is " (Utilities|String|ToString(Integer) Elapsed)))
  (|SetBy-RefVar (stale _canvas))
  (bind _canvas (Class|AgoraRtcEngine|SetupLocalVideo (Variables|Default|GetRtcEngine))))

(fn OnUserOffline
  (params (Uid :type Integer64) (Reason :type EUSER_OFFLINE_REASON_TYPE%20Enum :default "USER_OFFLINE_QUIT"))
  (Development|PrintString (Utilities|String|Append "user offline is" (Utilities|String|ToString(Text) (Utilities|Text|ToText(String) Uid))))
  (LocalVariables|Setremoteuid Uid)
  (|SetBy-RefVar (stale _canvas) (Utilities|Struct|MakeVideoCanvas 0 "RENDER_MODE_HIDDEN" "VIDEO_MIRROR_MODE_AUTO" (LocalVariables|Getremoteuid) false "VIDEO_SOURCE_REMOTE"))
  (|SetBy-RefVar (stale _connection) (Utilities|Struct|MakeRtcConnection (Variables|Default|GetChannelId) (LocalVariables|Getremoteuid)))
  (bind (_canvas _connection) (Class|AgoraRtcEngine|SetupRemoteVideoEx (Variables|Default|GetRtcEngine))))

(fn OnLeaveChannel
  (params (Stats :type Rtc%20Stats%20Structure%20%28by%20ref%29)))

(fn BindEvent
  (EventDispatchers|BindEventtoOnUserJoined (Variables|Default|GetEventHandler) (EventDispatchers|CreateEvent :!event OnUserJoinCallBack))
  (EventDispatchers|BindEventtoOnLeaveChannel (Variables|Default|GetEventHandler) (EventDispatchers|CreateEvent :!event OnLeaveChannel))
  (EventDispatchers|BindEventtoOnUserOffline (Variables|Default|GetEventHandler) (EventDispatchers|CreateEvent :!event OnUserOffline))
  (EventDispatchers|BindEventtoOnJoinChannelSuccess (Variables|Default|GetEventHandler) (EventDispatchers|CreateEvent :!event OnUserJoinChannelSuccess)))

(fn BasicAudioCallSceneBackHome
  (Game|OpenLevel(byObjectReference) "/Game/API-Example/MainLevel.MainLevel"))

(fn CheckPermission
  (if (Utilities|Enum|Equal(Enum) (Game|GetPlatformName) "Android")
    (Class|AndroidPermissionFunctionLibrary|AcquirePermissions (Utilities|Array|MakeArray "android.permission.RECORD_AUDIO" "android.permission.READ_PHONE_STATE" "android.permission.WRITE_EXTERNAL_STORAGE"))))

(fn InitRtcEngine
  (bind _returnvalue (Game|SpawnActorfromClass "/Script/AgoraPlugin.AgoraRtcEngine" (Math|Transform|MakeTransform "0, 0, 0" "0, 0, 0" "1.000000,1.000000,1.000000") "Undefined" 0 0))
  (Variables|Default|SetRtcEngine _returnvalue)
  (bind _returnvalue_2 (Game|SpawnActorfromClass "/AgoraPlugin/IRtcEngineEventHandler.IRtcEngineEventHandler_C" (Math|Transform|MakeTransform "0, 0, 0" "0, 0, 0" "1.000000,1.000000,1.000000") "Undefined" 0 0))
  (bind _output_get (Variables|Default|SetEventHandler _returnvalue_2))
  (CallFunction|BindEvent)
  (|SetBy-RefVar (stale _context) (Utilities|Struct|MakeRtcEngineContext (Variables|Default|GetAppid) _output_get 0 "CHANNEL_PROFILE_LIVE_BROADCASTING" "AUDIO_SCENARIO_DEFAULT" "AGORA_NULL_VALUE" "NORMAL" "(filePath=\"\",fileSizeInKB=1024,level=LOG_LEVEL_INFO)" "AREA_CODE_GLOB"))
  (bind (_context _returnvalue_3) (Class|AgoraRtcEngine|Initialize (Variables|Default|GetRtcEngine)))
  (Development|PrintString (Utilities|String|Append "initRtcEngine is" (Utilities|String|ToString(Integer) _returnvalue_3))))